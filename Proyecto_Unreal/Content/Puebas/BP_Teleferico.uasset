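; Cable car actor that travels along a spline path in the level and has a sliding door.
; TrainActivation checks an Integracion counter, finds the SplinePathBP actor, and starts a timeline that maps its alpha to spline distance for position and rotation.
; StationArrived and StationFinal print debug messages and stop that movement timeline.
; OpenDoorCableway runs a second timeline that slides the door sideways.
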(event `self.ReceiveBeginPlay`)

(event `/Game/Puebas/BPI_Estacion.Train Activation`
  (if (<= (`self.Integracion`) 2)
    (bind _returnvalue (`GameplayStatics.GetActorOfClass` "/Game/Puebas/SplinePathBP.SplinePathBP_C"))
    (set `self.Path` _returnvalue)
    (`self.Mov_Objet`)))

(event `Mov_Objet`
  (bind (_direction _alpha) (`Timeline|Timeline` :!label _label)
    (:`Update`
      (bind (_returnvalue_location _returnvalue_rotation) (`KismetMathLibrary.BreakTransform` (`SplineComponent.GetTransformAtDistanceAlongSpline` (`/Game/Puebas/SplinePathBP.Spline` (`self.Path`)) (`KismetMathLibrary.Lerp` 0.0 (`SplineComponent.GetSplineLength` (`/Game/Puebas/SplinePathBP.Spline` (`self.Path`))) _alpha) "World" false)))
      (`self.K2_SetActorLocationAndRotation` _returnvalue_location _returnvalue_rotation))))

(event `/Game/Puebas/BPI_Estacion.Station Arrived`
  (`KismetSystemLibrary.PrintString` "CableWay Stop")
  (set `self.Integracion` (`self.Integracion`) :!label _label_2)
  (goto _label :!via `Stop`))

(event `/Game/Puebas/BPI_Estacion.Station Final`
  (`KismetSystemLibrary.PrintString` "Station Final")
  (goto _label_2))

(event `/Game/Puebas/BPI_Estacion.Open Door Cableway`
  (`KismetSystemLibrary.PrintString` "Door CableWay")
  (bind (_direction _alpha) (`Timeline|Time_Door`)
    (:`Update`
      (`SceneComponent.K2_SetRelativeLocation` (`self.Door`) (`KismetMathLibrary.VLerp` (0.0 0.0 -400.0) (-400.0 0.0 -400.0) _alpha) false false))))

(fn `UserConstructionScript`)