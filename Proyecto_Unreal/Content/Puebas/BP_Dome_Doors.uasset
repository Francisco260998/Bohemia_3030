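; BP_Dome_Doors is a pair of sliding doors that open and close for the BP_Teleferico cable car.
; Overlap of the Collicion_Open trigger by the cable car plays a timeline that lerps both door halves' relative locations apart along X.
; Overlap of the separate Collicion_Close trigger reverses the same timeline to shut them.
; Both triggers ignore other actors and print a debug string.
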(event `self.Collicion_Open.OnComponentBeginOverlap`
  (params (OverlappedComponent :type "PrimitiveComponent Object Reference") (OtherActor :type "Actor Object Reference") (OtherComp :type "PrimitiveComponent Object Reference") (OtherBodyIndex :type Integer) (bFromSweep :type Boolean) (SweepResult :type "HitResult Structure (by ref)"))
  (cast `/Game/Puebas/BP_Teleferico` OtherActor)
  (`KismetSystemLibrary.PrintString` "Teleferic passed")
  (bind (_direction _alpha) (`Timeline|Timeline` :!label _label)
    (:`Update`
      (`SceneComponent.K2_SetRelativeLocation` (`self.Door_Left`) (`KismetMathLibrary.VLerp` (-40.0 0.0 0.0) (-150.0 0.0 0.0) _alpha) false false)
      (`SceneComponent.K2_SetRelativeLocation` (`self.Door_Right`) (`KismetMathLibrary.VLerp` (40.0 0.0 0.0) (150.0 0.0 0.0) _alpha) false false))))

(event `self.Collicion_Close.OnComponentBeginOverlap`
  (params (OverlappedComponent :type "PrimitiveComponent Object Reference") (OtherActor :type "Actor Object Reference") (OtherComp :type "PrimitiveComponent Object Reference") (OtherBodyIndex :type Integer) (bFromSweep :type Boolean) (SweepResult :type "HitResult Structure (by ref)"))
  (cast `/Game/Puebas/BP_Teleferico` OtherActor)
  (`KismetSystemLibrary.PrintString` "Close Door")
  (goto _label :!via `Reverse`))

(fn `UserConstructionScript`)